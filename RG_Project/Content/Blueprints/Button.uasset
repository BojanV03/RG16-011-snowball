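; Weight-activated pressure button that switches a target actor on or off depending on the physics balls resting on it.
; Box overlap events add or subtract each PhysicsBallBP's mass from a running total and print it as debug text.
; Both events share one threshold check that lowers the button and sends ActivateMessage above ActivationWeight, otherwise raises it and sends DeactivateMessage.
; Messages go through the ButtonActivated interface, so any implementing actor can be the target.
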(event OnComponentBeginOverlap(Box)
  (params (OverlappedComponent :type Primitive%20Component%20Object%20Reference) (OtherActor :type Actor%20Object%20Reference) (OtherComp :type Primitive%20Component%20Object%20Reference) (OtherBodyIndex :type Integer) (bFromSweep :type Boolean) (SweepResult :type Hit%20Result%20Structure%20%28by%20ref%29))
  (bind _target (Variables|Default|GetTarget))
  (bind _target_2 (Variables|Default|GetTarget))
  (bind _asphysics_ball_bp (Utilities|Casting|CastToPhysicsBallBP OtherActor))
  (bind _output_get (Variables|Default|SetCurrentWeight (+ (Variables|Default|GetCurrentWeight) (Physics|GetMass (Variables|/Game/RollingBP/Blueprints/PhysicsBallBP.PhysicsBallBP_C|GetBall _asphysics_ball_bp)))))
  (Development|PrintText (Utilities|Text|ToText(String) (|MakeString _output_get)) true true "(R=1.000000,G=0.500000,B=0.000000,A=1.000000)")
  (if (> (Variables|Default|GetCurrentWeight) (Variables|Default|GetActivationWeight))
    (Transformation|SetRelativeLocation (Variables|Default|GetButton) "0, 0,-5.000000" true false)
    (if (Utilities|DoesObjectImplementInterface _target_2 "/Game/Blueprints/ButtonActivated.ButtonActivated_C")
      (Class|ButtonActivated|Activate(Message) _target_2))
    (else
      (Transformation|SetRelativeLocation (Variables|Default|GetButton) "0, 0,0.000000" true false)
      (if (Utilities|DoesObjectImplementInterface _target "/Game/Blueprints/ButtonActivated.ButtonActivated_C")
        (Class|ButtonActivated|Deactivate(Message) _target)))))

(event OnComponentEndOverlap(Box)
  (params (OverlappedComponent :type Primitive%20Component%20Object%20Reference) (OtherActor :type Actor%20Object%20Reference) (OtherComp :type Primitive%20Component%20Object%20Reference) (OtherBodyIndex :type Integer))
  (bind _target (Variables|Default|GetTarget))
  (bind _target_2 (Variables|Default|GetTarget))
  (bind _asphysics_ball_bp (Utilities|Casting|CastToPhysicsBallBP OtherActor))
  (bind _output_get (Variables|Default|SetCurrentWeight (- (Variables|Default|GetCurrentWeight) (Physics|GetMass (Variables|/Game/RollingBP/Blueprints/PhysicsBallBP.PhysicsBallBP_C|GetBall _asphysics_ball_bp)))))
  (Development|PrintText (Utilities|Text|ToText(String) (|Makestring _output_get)) true true "(R=1.000000,G=0.493580,B=0.000000,A=1.000000)")
  (if (> (Variables|Default|GetCurrentWeight) (Variables|Default|GetActivationWeight))
    (Transformation|SetRelativeLocation (Variables|Default|GetButton) "0, 0,-5.000000" true false)
    (if (Utilities|DoesObjectImplementInterface _target_2 "/Game/Blueprints/ButtonActivated.ButtonActivated_C")
      (Class|ButtonActivated|Activate(Message) _target_2))
    (else
      (Transformation|SetRelativeLocation (Variables|Default|GetButton) "0, 0,0.000000" true false)
      (if (Utilities|DoesObjectImplementInterface _target "/Game/Blueprints/ButtonActivated.ButtonActivated_C")
        (Class|ButtonActivated|Deactivate(Message) _target)))))

(event EventBeginPlay)

(event Collision|EventActorBeginOverlap
  (params (OtherActor :type Actor%20Object%20Reference)))

(event EventTick
  (params (DeltaSeconds :type Float%20%28single-precision%29)))

(fn ConstructionScript)