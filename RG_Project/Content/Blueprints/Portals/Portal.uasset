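; Portal actor that teleports any overlapping actor to the plane of its linked TargetPortal.
; Before moving the actor, it disables teleporting on the target for one second to prevent an immediate bounce back.
; Each tick, its scene capture follows the player camera, offset by the vector between the two planes and copying camera rotation without compensating for portal orientation.
; BeginPlay caches the player pawn as a PhysicsBallBP.
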(event OnComponentBeginOverlap(Plane)
  (params (OverlappedComponent :type Primitive%20Component%20Object%20Reference) (OtherActor :type Actor%20Object%20Reference) (OtherComp :type Primitive%20Component%20Object%20Reference) (OtherBodyIndex :type Integer) (bFromSweep :type Boolean) (SweepResult :type Hit%20Result%20Structure%20%28by%20ref%29))
  (bind _targetportal (Variables|Default|GetTargetPortal))
  (if (Variables|Default|GetcanTeleport)
    (Utilities|DisableTeleport _targetportal)
    (Development|PrintText "Hello")
    (if true
      (Transformation|SetActorLocation OtherActor (Transformation|GetWorldLocation (Variables|Portal_C|GetPlane _targetportal)) false true))))

(event Collision|EventActorBeginOverlap
  (params (OtherActor :type Actor%20Object%20Reference)))

(event EventTick
  (params (DeltaSeconds :type Float%20%28single-precision%29))
  (bind _returnvalue (Game|GetPlayerController 0))
  (bind _playercameramanager (Variables|/Script/Engine.PlayerController|GetPlayerCameraManager _returnvalue))
  (bind _transformcomponent (Variables|/Script/Engine.PlayerCameraManager|GetTransformComponent _playercameramanager))
  (Transformation|SetWorldLocationAndRotation (Variables|/Script/Engine.SceneCapture2D|GetCaptureComponent2D (Variables|Default|GetPortalView)) (+ (- (Transformation|GetWorldLocation (Variables|Portal_C|GetPlane (Variables|Default|GetTargetPortal))) (Transformation|GetWorldLocation (Variables|Default|GetPlane))) (Transformation|GetWorldLocation _transformcomponent)) (Transformation|GetWorldRotation _transformcomponent) false false))

(event EventBeginPlay
  (bind _asphysics_ball_bp (Utilities|Casting|CastToPhysicsBallBP (Game|Player|GetPlayerPawn 0))
    (:then
      (Variables|Default|SetBall _asphysics_ball_bp))
    (:CastFailed
      (Development|PrintText "PortalEventBegin: FailedCast" true true "(R=1.000000,G=0.000000,B=0.000000,A=1.000000)" 1e+01))))

(fn ConstructionScript)