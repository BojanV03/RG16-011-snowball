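; Stair actor that rises into view when something enters its Detection volume and sinks back when the volume empties.
; An overlap counter, shown on a text component every Tick, decides when to reverse the motion.
; The timeline acts as an update loop: its direction becomes a ±1 sign for a fixed Z step per update.
; Height checks stop the movement at the top, and reset and hide the stair at the bottom.
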(event OnComponentBeginOverlap(Detection)
  (params (OverlappedComponent :type Primitive%20Component%20Object%20Reference) (OtherActor :type Actor%20Object%20Reference) (OtherComp :type Primitive%20Component%20Object%20Reference) (OtherBodyIndex :type Integer) (bFromSweep :type Boolean) (SweepResult :type Hit%20Result%20Structure%20%28by%20ref%29))
  (bind _stair (Variables|Default|GetStair))
  (bind _stair_2 (Variables|Default|GetStair))
  (bind _stair_3 (Variables|Default|GetStair))
  (bind _relativelocation (Variables|/Script/Engine.SceneComponent|GetRelativeLocation _stair_2))
  (bind _relativelocation_2 (Variables|/Script/Engine.SceneComponent|GetRelativeLocation _stair_3))
  (Math|Integer|IncrementInt (Variables|Default|Getcontains)
    (:%20%20
      (Development|SetHiddeninGame (Variables|Default|GetStair) false true)
      (if (not (> (.z (Variables|/Script/Engine.SceneComponent|GetRelativeLocation (Variables|Default|GetStair))) 2e+02))
        (bind _direction (Timeline|Timeline_0 Play)
          (:Update
            (Transformation|SetRelativeLocation _stair (Math|Vector|MakeVector (.RelativeLocation_X (|NewLocation _stair (|Directionto+-1 _direction))) (.RelativeLocation_Y (|NewLocation _stair (|Directionto+-1 _direction))) (.ReturnValue (|NewLocation _stair (|Directionto+-1 _direction)))) false false)
            (if (> (.z _relativelocation_2) 2e+02)
              (Timeline|Timeline_0 Stop)
              (elif (< (.z _relativelocation_2) 9.0)
                (Transformation|SetRelativeLocation _stair_2 (Math|Vector|MakeVector (.x _relativelocation) (.y _relativelocation) 0.0) false false)
                (Development|SetHiddeninGame _stair_2 true true)
                (Timeline|Timeline_0 Stop)))))))))

(event OnComponentEndOverlap(Detection)
  (params (OverlappedComponent :type Primitive%20Component%20Object%20Reference) (OtherActor :type Actor%20Object%20Reference) (OtherComp :type Primitive%20Component%20Object%20Reference) (OtherBodyIndex :type Integer))
  (bind _stair (Variables|Default|GetStair))
  (bind _stair_2 (Variables|Default|GetStair))
  (bind _stair_3 (Variables|Default|GetStair))
  (bind _relativelocation (Variables|/Script/Engine.SceneComponent|GetRelativeLocation _stair_2))
  (bind _relativelocation_2 (Variables|/Script/Engine.SceneComponent|GetRelativeLocation _stair_3))
  (bind _result (Math|Integer|DecrementInt (Variables|Default|Getcontains))
    (:%20%20
      (if (== _result 0)
        (bind _direction (Timeline|Timeline_0 Reverse)
          (:Update
            (Transformation|SetRelativeLocation _stair (Math|Vector|MakeVector (.RelativeLocation_X (|NewLocation _stair (|Directionto+-1 _direction))) (.RelativeLocation_Y (|NewLocation _stair (|Directionto+-1 _direction))) (.ReturnValue (|NewLocation _stair (|Directionto+-1 _direction)))) false false)
            (if (> (.z _relativelocation_2) 2e+02)
              (Timeline|Timeline_0 Stop)
              (elif (< (.z _relativelocation_2) 9.0)
                (Transformation|SetRelativeLocation _stair_2 (Math|Vector|MakeVector (.x _relativelocation) (.y _relativelocation) 0.0) false false)
                (Development|SetHiddeninGame _stair_2 true true)
                (Timeline|Timeline_0 Stop)))))))))

(event EventBeginPlay)

(event Collision|EventActorBeginOverlap
  (params (OtherActor :type Actor%20Object%20Reference)))

(event EventTick
  (params (DeltaSeconds :type Float%20%28single-precision%29))
  (Rendering|Components|TextRender|SetText (Variables|Default|GetText) (Utilities|Text|ToText(Integer) (Variables|Default|Getcontains))))

(fn ConstructionScript)