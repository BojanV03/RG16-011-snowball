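; WarmArea is a heat zone that gradually resizes any PhysicsBallBP inside it, shrinking it when HeatIndex is positive.
; Collision overlap events add balls to BallArray on entry and remove them on exit, printing each in red debug text.
; Tick calls Resize on every tracked ball with a small negative amount scaled by DeltaSeconds and HeatIndex.
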(event OnComponentBeginOverlap(Collision)
  (params (OverlappedComponent :type Primitive%20Component%20Object%20Reference) (OtherActor :type Actor%20Object%20Reference) (OtherComp :type Primitive%20Component%20Object%20Reference) (OtherBodyIndex :type Integer) (bFromSweep :type Boolean) (SweepResult :type Hit%20Result%20Structure%20%28by%20ref%29))
  (bind _asphysics_ball_bp (Utilities|Casting|CastToPhysicsBallBP OtherActor))
  (Development|PrintText (Utilities|Text|ToText(String) (Utilities|String|ToString(Object) _asphysics_ball_bp)) true true "(R=1.000000,G=0.000000,B=0.000000,A=1.000000)")
  (Utilities|Array|AddUnique (Variables|Default|GetBallArray) _asphysics_ball_bp))

(event OnComponentEndOverlap(Collision)
  (params (OverlappedComponent :type Primitive%20Component%20Object%20Reference) (OtherActor :type Actor%20Object%20Reference) (OtherComp :type Primitive%20Component%20Object%20Reference) (OtherBodyIndex :type Integer))
  (bind _asphysics_ball_bp (Utilities|Casting|CastToPhysicsBallBP OtherActor))
  (Development|PrintText (Utilities|Text|ToText(String) (Utilities|String|ToString(Object) _asphysics_ball_bp)) true true "(R=1.000000,G=0.000000,B=0.000000,A=1.000000)")
  (Utilities|Array|RemoveItem (Variables|Default|GetBallArray) _asphysics_ball_bp))

(event EventBeginPlay)

(event Collision|EventActorBeginOverlap
  (params (OtherActor :type Actor%20Object%20Reference)))

(event EventTick
  (params (DeltaSeconds :type Float%20%28single-precision%29))
  (for _array_element (Variables|Default|GetBallArray)
    (Default|Resize _array_element (* DeltaSeconds -0.001 (Variables|Default|GetHeatIndex)))))

(fn ConstructionScript)