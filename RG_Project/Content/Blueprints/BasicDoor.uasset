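; BasicDoor is a door actor that slides its Cube up on Activate and back down on Deactivate, guarded by an Open flag.
; Two timelines act as update tickers, nudging the Cube's relative Z by a fixed step until it passes an upper or lower limit.
; Each event stops the opposing timeline, so movement can reverse midway, and prints an opening or closing message with the actor's name.
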(event EventBeginPlay)

(event Collision|EventActorBeginOverlap
  (params (OtherActor :type Actor%20Object%20Reference)))

(event EventDeactivate
  (bind (_cube _relativelocation_x _relativelocation_y _returnvalue) (|GetLocation 2.0))
  (bind (_cube_2 _relativelocation_x_2 _relativelocation_y_2 _returnvalue_2) (|GetLocation_2 -2.0))
  (if (Variables|Default|GetOpen)
    (Variables|Default|SetOpen false)
    (Utilities|FlowControl|Sequence
      (:then_0
        (Timeline|Timeline1 Stop
          (:Update
            (Transformation|SetRelativeLocation _cube (Math|Vector|MakeVector _relativelocation_x _relativelocation_y _returnvalue) false false)
            (if (> _returnvalue 2.8e+02)
              (Timeline|Timeline1 Stop)))))
      (:then_1
        (Timeline|Timeline_0 Play
          (:Update
            (Transformation|SetRelativeLocation _cube_2 (Math|Vector|MakeVector _relativelocation_x_2 _relativelocation_y_2 _returnvalue_2) false false)
            (if (< _returnvalue_2 8e+01)
              (Timeline|Timeline_0 Stop)))))
      (:then_2
        (|LogClose)))))

(event EventTick
  (params (DeltaSeconds :type Float%20%28single-precision%29)))

(event EventActivate
  (bind (_cube _relativelocation_x _relativelocation_y _returnvalue) (|GetLocation 2.0))
  (bind (_cube_2 _relativelocation_x_2 _relativelocation_y_2 _returnvalue_2) (|GetLocation_2 -2.0))
  (if (not (Variables|Default|GetOpen))
    (Variables|Default|SetOpen true)
    (Utilities|FlowControl|Sequence
      (:then_0
        (Timeline|Timeline1 PlayFromStart
          (:Update
            (Transformation|SetRelativeLocation _cube (Math|Vector|MakeVector _relativelocation_x _relativelocation_y _returnvalue) false false)
            (if (> _returnvalue 2.8e+02)
              (Timeline|Timeline1 Stop)))))
      (:then_1
        (Timeline|Timeline_0 Stop
          (:Update
            (Transformation|SetRelativeLocation _cube_2 (Math|Vector|MakeVector _relativelocation_x_2 _relativelocation_y_2 _returnvalue_2) false false)
            (if (< _returnvalue_2 8e+01)
              (Timeline|Timeline_0 Stop)))))
      (:then_2
        (|LogOpen)))))

(fn ConstructionScript)